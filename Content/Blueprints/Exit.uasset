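; Exit is a trigger actor that marks when the player character is leaving a ladder.
; On begin and end overlap it casts the other actor to GAME_PRODUCTION_IIICharacter and sets its IsLeaveingLadder flag true on entry and false on exit.
; Each change prints the flag's value to the screen as orange debug text.
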(event `self.ReceiveActorBeginOverlap`
  (params (OtherActor :type "Actor Object Reference"))
  ;[1 1 1] Begin overlap
  (bind _asgame_production_iiicharacter (cast `GAME_PRODUCTION_IIICharacter` OtherActor))
  (bind _output_get (set `GAME_PRODUCTION_IIICharacter.IsLeaveingLadder` true _asgame_production_iiicharacter))
  (`KismetSystemLibrary.PrintString` (`KismetStringLibrary.Concat_StrStr` "Is Leaveing Ladder ->" (`KismetStringLibrary.Conv_BoolToString` _output_get)) true true (struct :`R` 1.0 :`G` 0.574347 :`A` 1.0)))

(event `self.ReceiveActorEndOverlap`
  (params (OtherActor :type "Actor Object Reference"))
  ;[1 1 1] End overlap
  (bind _asgame_production_iiicharacter (cast `GAME_PRODUCTION_IIICharacter` OtherActor))
  (bind _output_get (set `GAME_PRODUCTION_IIICharacter.IsLeaveingLadder` false _asgame_production_iiicharacter))
  (`KismetSystemLibrary.PrintString` (`KismetStringLibrary.Concat_StrStr` "Is Leaveing Ladder ->" (`KismetStringLibrary.Conv_BoolToString` _output_get)) true true (struct :`R` 1.0 :`G` 0.574347 :`A` 1.0)))

(fn `UserConstructionScript`)